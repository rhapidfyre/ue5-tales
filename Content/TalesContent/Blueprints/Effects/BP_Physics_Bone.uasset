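; Physics bone debris actor that tumbles, makes noise on landing and removes itself after a set lifetime.
; On BeginPlay it applies the supplied mesh or a cracked-bone default.
; The authority then adds a jittered angular impulse about the up axis, randomizes rotation, waits, and shrinks the mesh by timeline before destroying the actor.
; Hard hits on Landscape play a random bone sound.
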(event `self.ReceiveBeginPlay`
  (bind _staticmesh (`self.StaticMesh`))
  (`|ExecutionSequence`
    (:`then_0`
      (bind _usebonemesh (`self.UseBoneMesh`)
        (:`then`
          (`StaticMeshComponent.SetStaticMesh` _staticmesh _usebonemesh))
        (:`else`
          (`StaticMeshComponent.SetStaticMesh` _staticmesh "/Game/PolygonDungeons/Meshes/Environments/Bones/SM_Env_Bone_Cracked_01.SM_Env_Bone_Cracked_01"))))
    (:`then_1`
      (`/Engine/EditorBlueprintResources/ActorMacros.Switch Has Authority`
        (:`Authority`
          (`PrimitiveComponent.AddAngularImpulseInDegrees` (`self.StaticMesh`) (* (+ (`self.GetActorUpVector`) (`KismetMathLibrary.MakeVector` (`KismetMathLibrary.RandomFloatInRange` -0.2 0.2) (`KismetMathLibrary.RandomFloatInRange` -0.2 0.2))) (`self.ImpulseStrength`)) "None" false)
          (`SceneComponent.K2_SetWorldRotation` (`self.StaticMesh`) (`KismetMathLibrary.RandomRotator` true) false false)
          (`KismetSystemLibrary.Delay` (`self.BoneLifetime`))
          (bind (_direction _newtrack_0) (`Timeline|FadeOutAndDie`)
            (:`Update`
              (`SceneComponent.SetWorldScale3D` (`self.StaticMesh`) (* (0.04 0.04 0.04) _newtrack_0)))
            (:`Finished`
              (`self.K2_DestroyActor`))))))))

(event `self.StaticMesh.OnComponentHit`
  (params (HitComponent :type "PrimitiveComponent Object Reference") (OtherActor :type "Actor Object Reference") (OtherComp :type "PrimitiveComponent Object Reference") (NormalImpulse :type "Vector Structure") (Hit :type "HitResult Structure (by ref)"))
  (cast `Landscape` OtherActor)
  (if (> (`KismetMathLibrary.VSize` NormalImpulse) 240.0)
    (`GameplayStatics.PlaySoundAtLocation` (`KismetArrayLibrary.Array_Random` (`self.BoneNoises`)) (`self.K2_GetActorLocation`) (struct) 0.4 1.0 0.0 null null null null)))

(fn `UserConstructionScript`)