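; AI controller for combat NPCs that picks enemies by faction standing and tracks them in a hate list.
; Sight or other perception events add or remove hate, weighting players higher, and a looping tick adjusts it.
; ProcessHateList writes a target from that list to the blackboard.
; An authority-only timer, stored as HateTimer, fires primary attacks in range, pausing randomly after each and whenever perception finds the list empty.
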(event `StopBehavior`
  (set `self.BehaviorTree` null))

(event `PerformAttack_Timer`
  (bind _hatetimer (`self.HateTimer`))
  (if (`self.IsInAttackRange`)
    (bind _returnvalue (`self.PerformAttack` "/Game/TalesContent/Inputs/Actions/IA_Attack_Primary.IA_Attack_Primary"))
    (if _returnvalue
      (`KismetSystemLibrary.K2_PauseTimerHandle` _hatetimer)
      (`KismetSystemLibrary.Delay` (`KismetMathLibrary.RandomFloatInRange` 3.0 5.0))
      (`KismetSystemLibrary.K2_UnPauseTimerHandle` _hatetimer))))

(event `Callback_PerceptionUpdate`
  (params (Actor :type "Actor Object Reference") (Stimulus :type "AIStimulus Structure"))
  (bind _hatetimer (`self.HateTimer`))
  (`|ExecutionSequence`
    (:`then_0`
      (if (`.bSuccessfullySensed` (break `AIStimulus` Stimulus))
        (bind _ascharacter_base (cast `CharacterBase` Actor))
        (`self.CheckTargetHate` _ascharacter_base)
        (else
          (bind _ascharacter_base_2 (cast `CharacterBase` Actor))
          (if (`BlueprintMapLibrary.Map_Contains` (`self.GetHateList`) _ascharacter_base_2)
            (bind _asplayer_character_base (cast `PlayerCharacterBase` _ascharacter_base_2)
              (:`then`
                (`self.RemoveHateFromTarget` _asplayer_character_base 2.0))
              (:`CastFailed`
                (`self.RemoveHateFromTarget` _ascharacter_base_2)))))))
    (:`then_1`
      (bind _keys (`BlueprintMapLibrary.Map_Keys` (`self.GetHateList`)))
      (if (> (`KismetArrayLibrary.Array_Length` _keys) 0)
        (`KismetSystemLibrary.K2_UnPauseTimerHandle` _hatetimer)
        (else
          (`KismetSystemLibrary.K2_PauseTimerHandle` _hatetimer))))))

(event `self.ReceiveBeginPlay`
  (`parent.ReceiveBeginPlay`)
  (`|ExecutionSequence`
    (:`then_0`
      (bind _ascombat_npc_character_base (cast `CombatNpcCharacterBase` (`self.K2_GetPawn`)))
      (set `self.ControlledCharacter` _ascombat_npc_character_base)
      (add `AIPerceptionComponent.OnTargetPerceptionUpdated` (`self.AiPerception`) (`|CreateDelegate` :!event `Callback_PerceptionUpdate`))
      (add `self.OnHateListUpdated` (`|CreateDelegate` :!event `ProcessHateList`))
      (`self.InitBehaviorTree`)
      (`KismetSystemLibrary.K2_SetTimerDelegate` (delegate `Callback_HateTick`) 1.0 true))
    (:`then_1`
      (`/Engine/EditorBlueprintResources/ActorMacros.Switch Has Authority`
        (:`Authority`
          (bind _returnvalue (`KismetSystemLibrary.K2_SetTimerDelegate` (delegate `PerformAttack_Timer`) 1.0 true))
          (set `self.HateTimer` _returnvalue))))))

(event `InitBehaviorTree`
  (cast `NpcCharacterBase` (`self.K2_GetPawn`)
    (:`CastFailed`
      (`KismetSystemLibrary.Delay` 0.2)
      (`self.InitBehaviorTree`))))

(event `Callback_HateTick`
  (bind _keys (`BlueprintMapLibrary.Map_Keys` (`self.GetHateList`)))
  (for _array_element _keys
    (if (`self.IsTargetValid` _array_element)
      (bind _ascharacter_base (cast `CharacterBase` _array_element))
      (`self.AddHateTowardsTarget` _ascharacter_base 2.0)))
  (`|ExecutionSequence`
    (:`then_0`
      (bind _keys_2 (`BlueprintMapLibrary.Map_Keys` (`self.GetHateList`)))
      (for _array_element_2 _keys_2
        (`self.RemoveHateFromTarget` _array_element_2)))))

(event `Callback_PatrolStatus`
  (params (IsPatrollingNpc :type Boolean))
  (bind _returnvalue (`AIBlueprintHelperLibrary.GetBlackboard` null))
  (`/Engine/EditorBlueprintResources/StandardMacros.IsValid` _returnvalue
    (:`Is Valid`
      (`BlackboardComponent.SetValueAsBool` _returnvalue "IsPatroller" IsPatrollingNpc))))

(fn `CheckTargetHate`
  (params (InActor :type "CharacterBase Object Reference"))
  (locals (tLowestValue :type "Float (double-precision)" :default 500.0) (tFactionMap :type "Map of EFaction Enum to StFactionData Structure") (tHasHate :type Boolean))
  (set `local.tHasHate` (`BlueprintMapLibrary.Map_IsNotEmpty` (`self.GetHateList`)))
  (for _array_element (`CharacterBase.FactionStandings` (`self.ControlledCharacter`))
    (set `local.tFactionMap` (`|MakeMap` (`.FactionEnum` (break `StFactionData` _array_element)) _array_element)))
  (for _array_element_2 (`CharacterBase.FactionMemberships` (`local.InActor`))
    (bind (_value _returnvalue) (`BlueprintMapLibrary.Map_Find` (`local.tFactionMap`) _array_element_2))
    (if _returnvalue
      (bind (_factionenum _factionvalue) (break `StFactionData` _value))
      (if (< _factionvalue (`local.tLowestValue`))
        (set `local.tLowestValue` _factionvalue))))
  (`|ExecutionSequence`
    (:`then_0`
      (if (< (`local.tLowestValue`) 0.0)
        (bind _asplayer_character_base (cast `PlayerCharacterBase` (`local.InActor`))
          (:`then`
            (`self.AddHateTowardsTarget` _asplayer_character_base 2.0) ; Players gain more initial hate than NPCs
          )
          (:`CastFailed`
            (`self.AddHateTowardsTarget` null) ; Pets, guards, mercenaries, etc.
          ))))
    (:`then_1`
      ;[0.2 0.2 0.2 0.4] Move to an interface
      (if (and (not (`local.tHasHate`)) (`BlueprintMapLibrary.Map_IsNotEmpty` (`self.GetHateList`)))
        (bind _controlledcharacter (`self.ControlledCharacter`)
          (:`then`
            (bind _asnpc_tormented_soul (cast `/Game/TalesContent/Blueprints/NPC/NPC_Tormented_Soul` _controlledcharacter))
            (`/Game/TalesContent/Blueprints/NPC/NPC_Tormented_Soul.PlayTaunt` _asnpc_tormented_soul))
          (:`else`))))))

(fn `ProcessHateList`
  (locals (tMostHatedTarget :type "CharacterBase Object Reference"))
  (bind _returnvalue (`AIBlueprintHelperLibrary.GetBlackboard` null))
  (bind _tmosthatedtarget (`local.tMostHatedTarget`))
  (bind _returnvalue_2 (`BlackboardComponent.GetValueAsObject` _returnvalue (`self.TargetActorBbKey`)))
  (bind _keys (`BlueprintMapLibrary.Map_Keys` (`self.GetHateList`)))
  (set `local.tMostHatedTarget` (`|GetArrayItem` _keys))
  (`self.ControlledCharacter`
    (:`then`
      (`/Engine/EditorBlueprintResources/StandardMacros.IsValid` _returnvalue
        (:`Is Valid`
          (`/Engine/EditorBlueprintResources/StandardMacros.IsValid` _tmosthatedtarget
            (:`Is Valid`
              (`/Engine/EditorBlueprintResources/StandardMacros.IsValid` _returnvalue_2
                (:`Is Valid`
                  (if (!= _returnvalue_2 _tmosthatedtarget)
                    (`BlackboardComponent.SetValueAsObject` _returnvalue (`self.TargetActorBbKey`) (`local.tMostHatedTarget`) :!label _label)))
                (:`Is Not Valid`
                  (goto _label))))
            (:`Is Not Valid`
              (`BlackboardComponent.ClearValue` _returnvalue (`self.TargetActorBbKey`)))))))
    (:`else`)))

(fn `UserConstructionScript`)