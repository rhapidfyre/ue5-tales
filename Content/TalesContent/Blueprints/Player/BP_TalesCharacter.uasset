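; Player character Blueprint that interrupts ability casting on input and shows a ring under the current target.
; Starting crouch, jump or move calls InterruptCasting on the AbilityComponent for focused casts only.
; The component's new-target callback spawns BP_TargetRing as needed, snaps it to the target mesh's root socket, or destroys it without a target.
; A timer-based ring location update remains, but its timer setup is disconnected.
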(event `self.ReceiveBeginPlay`
  (`parent.ReceiveBeginPlay`)
  (add `AbilityComponent.OnNewTargetSet` (`self.AbilityComponent`) (`|CreateDelegate` :!event `UpdateTargetRing`)))

(event `EnhancedInput|/Game/TalesContent/Inputs/Actions/IA_Crouch`
  (params (ActionValue :type Boolean) (ElapsedSeconds :type "Float (double-precision)") (TriggeredSeconds :type "Float (double-precision)") (InputAction :type "InputAction Object Reference" :default "/Game/TalesContent/Inputs/Actions/IA_Crouch.IA_Crouch"))
  (:`Started`
    (`AbilityComponent.InterruptCasting` (`self.AbilityComponent`) true false :!label _label)))

(event `EnhancedInput|/Game/TalesContent/Inputs/Actions/IA_Jump`
  (params (ActionValue :type Boolean) (ElapsedSeconds :type "Float (double-precision)") (TriggeredSeconds :type "Float (double-precision)") (InputAction :type "InputAction Object Reference" :default "/Game/TalesContent/Inputs/Actions/IA_Jump.IA_Jump"))
  (:`Started`
    (goto _label)))

(event `EnhancedInput|/Game/TalesContent/Inputs/Actions/IA_Move`
  (params (ActionValue :type "Vector2D Structure") (ElapsedSeconds :type "Float (double-precision)") (TriggeredSeconds :type "Float (double-precision)") (InputAction :type "InputAction Object Reference" :default "/Game/TalesContent/Inputs/Actions/IA_Move.IA_Move"))
  (:`Started`
    (goto _label)))

(event `UpdateTargetRing`
  (params (NewTarget :type "CharacterBase Object Reference"))
  (`KismetSystemLibrary.K2_ClearAndInvalidateTimerHandle` (`self.TargetTimer`))
  (`/Engine/EditorBlueprintResources/StandardMacros.IsValid` NewTarget
    (:`Is Valid`
      (`self.TargetRing`
        (:`then`
          _)
        (:`else`
          (bind _returnvalue (`|SpawnActorFromClass` "/Game/TalesContent/Blueprints/BP_TargetRing.BP_TargetRing_C" (`KismetMathLibrary.MakeTransform` (-90.0 0.0 0.0)) "AlwaysSpawn" "MultiplyWithRoot" null (struct :`R` 1.0 :`G` 1.0 :`B` 1.0 :`A` 0.1) null))
          (set `self.TargetRing` _returnvalue)))
      (`self.K2_AttachToComponent` (`self.TargetRing`) (`Character.Mesh` NewTarget) "root" "SnapToTarget" "KeepWorld" "KeepWorld" true))
    (:`Is Not Valid`
      (bind _targetring (`self.TargetRing`)
        (:`then`
          (`self.K2_DestroyActor` _targetring))
        (:`else`)))))

(event `UpdateTargetRingLocation`
  (bind (_returnvalue_location _returnvalue_rotation) (`KismetMathLibrary.BreakTransform` (`SceneComponent.GetSocketTransform` (`Character.Mesh` (`AbilityComponent.GetTargetedActor` (`self.AbilityComponent`))) "root" "RTS_World")))
  (bind _targetring (`self.TargetRing`)
    (:`then`
      (`self.K2_SetActorLocationAndRotation` _targetring _returnvalue_location (`KismetMathLibrary.MakeRotator` (+ (.roll _returnvalue_rotation) 90.0) (.pitch _returnvalue_rotation)) false true))
    (:`else`)))

(fn `UserConstructionScript`)