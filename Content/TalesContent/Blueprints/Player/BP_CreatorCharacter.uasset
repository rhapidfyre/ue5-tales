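; BP_CreatorCharacter is the creator character whose mesh visibility follows the character slot selected in BP_CreatorGameState.
; On BeginPlay it resets the game state's selection to 0, binds to OnCharacterSelected and applies the current selection.
; The selection callback hides the mesh for slot 0 and shows it for any other value.
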(event `self.ReceiveBeginPlay`
  (bind _asbp_creator_game_state (cast `/Game/TalesContent/Gamemode/Creation/BP_CreatorGameState` (`GameplayStatics.GetGameState`)))
  (`/Game/TalesContent/Gamemode/Creation/BP_CreatorGameState.SetSelectedCharacter` _asbp_creator_game_state 0)
  (add `/Game/TalesContent/Gamemode/Creation/BP_CreatorGameState.OnCharacterSelected` _asbp_creator_game_state (delegate `Callback_CharacterSelection`))
  (`self.Callback_CharacterSelection` (`/Game/TalesContent/Gamemode/Creation/BP_CreatorGameState.GetSelectedCharacterNumber` _asbp_creator_game_state)))

(event `Callback_CharacterSelection`
  (params (SaveSlotNumber :type Integer))
  (`/Engine/EditorBlueprintResources/StandardMacros.CompareInt` SaveSlotNumber
    (:`>`
      (`SceneComponent.SetVisibility` (`self.Mesh`) true false))
    (:`==`
      (`SceneComponent.SetVisibility` (`self.Mesh`) false false))
    (:`<`
      (`SceneComponent.SetVisibility` (`self.Mesh`) true false))))

(fn `UserConstructionScript`)