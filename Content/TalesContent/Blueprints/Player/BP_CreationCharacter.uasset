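; Character Blueprint for the character creator that caches the creator game state and HUD references on BeginPlay.
; It retries both casts every 0.2 seconds until they succeed, then binds to the HUD's creator-update event.
; Selection and update handlers are empty stubs.
; Logic toggling mesh visibility from save existence, selection and creator-open state is disconnected, as are the character selection and restore bindings.
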(event `self.ReceiveBeginPlay`
  (`parent.ReceiveBeginPlay`)
  (`self.InitGameState`))

(event `InitGameState`
  (bind _ascreator_game_state_base (cast `CreatorGameStateBase` (`GameplayStatics.GetGameState`))
    (:`then`
      (set `self.GameStateReference` _ascreator_game_state_base)
      (bind _asbp_creator_hud (cast `/Game/TalesContent/Gamemode/Creation/BP_CreatorHud` (`PlayerController.GetHUD` (`GameplayStatics.GetPlayerController` 0)))
        (:`then`
          (bind _output_get (set `self.HudReference` _asbp_creator_hud))
          (add `/Game/TalesContent/Gamemode/Creation/BP_CreatorHud.OnCreatorUpdate` _output_get (`|CreateDelegate` :!event `EventCreatorUpdate`)))
        (:`CastFailed`
          (`KismetSystemLibrary.Delay` 0.2 :!label _label)
          (`self.InitGameState`))))
    (:`CastFailed`
      (goto _label))))

(event `Callback_OnCharacterRestored`
  (params (bWasSuccess :type Boolean))
  (`self.Callback_CharacterSelection` 0))

(event `Callback_CharacterSelection`
  (params (SelectedIndex :type Integer)))

(event `EventCreatorUpdate`)

(fn `UserConstructionScript`
  (`parent.UserConstructionScript`))