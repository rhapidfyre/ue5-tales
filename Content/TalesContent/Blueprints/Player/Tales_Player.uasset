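; Player character Blueprint that manages interaction detection, targeting, camera switching and death feedback.
; Each tick, a camera-forward sphere trace against pawns messages hit actors and caches the interactive actor, exposed alongside the current target.
; The target clears itself when its AbilitySystemComponent reports death.
; Death and revive events swap follow and post-processed death cameras for the local player, with montage and sound feedback, while currency updates play a coin sound.
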(event `SetTargetActor`
  (params (TargetActor :type "CharacterBase Object Reference"))
  (`|ExecutionSequence`
    (:`then_0`
      (bind _targetactor (`self.TargetActor`)
        (:`then`
          (remove `RsAbilityComponent.OnDeathStatusChanged` (`CharacterBase.AbilitySystemComponent` _targetactor) (`|CreateDelegate` :!event `TargetActorDeath_Event`)))
        (:`else`)))
    (:`then_1`
      (bind _output_get (set `self.TargetActor` TargetActor))
      (`self.OnTargetUpdated` _output_get)
      (`/Engine/EditorBlueprintResources/StandardMacros.IsValid` _output_get
        (:`Is Valid`
          (add `RsAbilityComponent.OnDeathStatusChanged` (`CharacterBase.AbilitySystemComponent` _output_get) (`|CreateDelegate` :!event `TargetActorDeath_Event`)))))))

(event `self.ReceiveTick`
  (params (DeltaSeconds :type "Float (single-precision)"))
  (bind _returnvalue (`GameplayStatics.GetPlayerCameraManager` 0))
  (bind _returnvalue_2 (`self.K2_GetActorLocation` _returnvalue))
  (`parent.ReceiveTick` DeltaSeconds)
  (bind (_outhits _returnvalue_3) (`KismetSystemLibrary.SphereTraceMultiForObjects` :`Start` _returnvalue_2 :`End` (+ (* (`self.GetActorForwardVector` _returnvalue) 1000.0) _returnvalue_2) :`Radius` 12.0 :`ObjectTypes` (`|MakeArray` "ObjectTypeQuery3" :!type "EObjectTypeQuery Enum") :`DrawTime` 2.0))
  (if _returnvalue_3
    (for _array_element _outhits
      (bind (_bblockinghit _binitialoverlap _time _distance _location _impactpoint _normal _impactnormal _physmat _hitactor) (`GameplayStatics.BreakHitResult` _array_element))
      (message `/T5GInventorySystem/Game/InteractionInterface.ShowDataInterface` _hitactor 0.0)
      (bind _aboutobject (message `/T5GInventorySystem/Game/InteractionInterface.CheckInteractive` _hitactor))
      (set `self.InteractiveActor` _aboutobject))
    (else
      (set `self.InteractiveActor` null))))

(event `SetCharacterCamera`
  (params (CameraNumber :type Integer))
  (if (== CameraNumber 1)
    (`ActorComponent.Deactivate` (`self.FollowCamera`))
    (`ActorComponent.Activate` (`self.MenuCamera`) true)
    (else
      (`ActorComponent.Deactivate` (`self.MenuCamera`))
      (`ActorComponent.Activate` (`self.FollowCamera`) true))))

(event `MC_OnDeathStatus`
  (params (IsNowDead :type Boolean) (NewHealth :type "Float (double-precision)"))
  (if IsNowDead
    (`|PlayMontage` (`self.Mesh`) "/Game/Blink/Characters/LowPoly/Humans/Male/Anims/Anim_Death_Montage.Anim_Death_Montage")))

(event `self.ReceiveBeginPlay`
  (`parent.ReceiveBeginPlay`)
  (`|ExecutionSequence`
    (:`then_0`
      (set `CameraComponent.PostProcessSettings` (`self.DeathPostProcessSettings`) (`self.DeathCamera`))
      (add `RsAbilityComponent.OnDeathStatusChanged` (`self.AbilitySystemComponent`) (`|CreateDelegate` :!event `MC_OnDeathStatus`)))
    (:`then_1`
      (add `InventoryComponent.OnCurrencyUpdated` (`self.InventoryComponent`) (`|CreateDelegate` :!event `Callback_CurrencyUpdated`)))))

(event `self.CharacterDeath`
  (if (`self.IsLocallyControlled`)
    (`GameplayStatics.PlaySound2D` "/Game/TalesContent/Music/CUE_Death_Title.CUE_Death_Title" 1.0 1.0 0.0 null null)
    (`ActorComponent.Activate` (`self.DeathCamera`) true)
    (`ActorComponent.Deactivate` (`self.FollowCamera`))
    (else
      (`GameplayStatics.PlaySoundAtLocation` "/Game/TalesContent/Sounds/death_bell_1.death_bell_1" (`self.K2_GetActorLocation`) (struct) 1.0 1.0 0.0 "/T5GInventorySystem/Audio/ATTN_PickupEffect.ATTN_PickupEffect" null null null))))

(event `self.CharacterRevived`
  (`|ExecutionSequence`
    (:`then_1`
      (if (`self.IsLocallyControlled`)
        (`|ExecutionSequence`
          (:`then_0`
            (`ActorComponent.Activate` (`self.FollowCamera`) true)
            (`ActorComponent.Deactivate` (`self.DeathCamera`))))))))

(event `Callback_CurrencyUpdated`
  (`GameplayStatics.PlaySound2D` "/Game/TalesContent/Sounds/Misc/coins_drop_1.coins_drop_1" 0.4 1.0 0.0 null null))

(event `TargetActorDeath_Event`
  (params (bIsNowDead :type Boolean) (CurrentHealth :type "Float (single-precision)"))
  (if bIsNowDead
    (`self.SetTargetActor` null)))

(fn `GetInteractiveActor`
  (returns (InteractiveActor :type "Object Object Reference"))
  (return (`self.InteractiveActor`)))

(fn `GetTargetedActor`
  (returns (HasTarget :type Boolean) (Target :type "CharacterBase Object Reference"))
  (bind _targetactor (`self.TargetActor`))
  (return (`KismetSystemLibrary.IsValid` _targetactor) _targetactor))

(fn `UserConstructionScript`
  (`parent.UserConstructionScript`))