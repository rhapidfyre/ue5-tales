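; BP_NPC_Spawner is a spawner actor that randomly places a single NPC at its own location and rotation.
; DetermineSpawn rolls against SpawnChance when no valid NPC reference exists, then spawns a random class from EligibleNpcs, adjusting for collisions, and stores the reference.
; DoSpawnEvent starts a short timer delay, and DoDespawnEvent destroys the stored NPC.
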(event Custom|DetermineSpawn
  (bind _returnvalue (Transformation|GetActorTransform))
  (Variables|Default|GetNpcReference
    (:then)
    (:else
      (if (<= (Math|Random|RandomFloatinRange 0.0 1.0) (Variables|SpawnerSettings|GetSpawnChance))
        (bind _returnvalue_2 (Game|SpawnActorfromClass (.OutItem (Utilities|Array|Random (Variables|SpawnerSettings|GetEligibleNpcs))) (Math|Transform|MakeTransform (.location _returnvalue) (.rotation _returnvalue) "1.000000,1.000000,1.000000") "AdjustIfPossibleButAlwaysSpawn" "MultiplyWithRoot" 0 0))
        (Variables|Default|SetNpcReference _returnvalue_2)))))

(event EventDoSpawnEvent
  (Utilities|Time|SetTimerbyEvent (EventDispatchers|CreateEvent :!event Custom|DetermineSpawn) 0.5))

(event EventDoDespawnEvent
  (bind _npcreference (Variables|Default|GetNpcReference)
    (:then
      (Actor|DestroyActor _npcreference))
    (:else)))

(fn ConstructionScript)