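; Blueprint for the Tormented Soul NPC, a character with an overhead widget and its own death effects.
; On BeginPlay it runs the parent logic and hands itself to the overhead widget as character reference.
; CharacterDeath plays a montage and random grunt, hides the widget, then fires a delayed explosion effect and sound.
; A parallel sequence branch hides the mesh without waiting for that delay and detaches any BP_CombatAi controller.
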(event `self.ReceiveBeginPlay`
  (`parent.ReceiveBeginPlay`)
  (bind _aswidget_overhead_player_data (cast `/Game/TalesContent/Widgets/Targeting/Widget_Overhead_PlayerData` (`WidgetComponent.GetWidget` (`self.Widget`))))
  (`/Game/TalesContent/Widgets/Targeting/Widget_Overhead_PlayerData.SetCharacterReference` _aswidget_overhead_player_data self))

(event `self.CharacterDeath`
  (bind _returnvalue (`self.K2_GetActorLocation`))
  (`|ExecutionSequence`
    (:`then_1`
      (`self.PlayAnimMontage` (`self.DeathMontage`))
      (`GameplayStatics.PlaySoundAtLocation` (`KismetArrayLibrary.Array_Random` (`|MakeArray` "/Game/HumanVocalizations/HumanMaleA/Cues/voice_male_grunt_pain_death_09_Cue.voice_male_grunt_pain_death_09_Cue" "/Game/HumanVocalizations/HumanMaleA/Cues/voice_male_grunt_pain_death_01_Cue.voice_male_grunt_pain_death_01_Cue" :!type "SoundBase Object Reference")) _returnvalue (struct) 1.0 1.0 0.0 null null null null)
      (`SceneComponent.SetVisibility` (`self.Widget`) false true)
      (`KismetSystemLibrary.Delay` 1.1)
      (`ActorComponent.Activate` (`self.Death_Fx`) true)
      (`GameplayStatics.PlaySoundAtLocation` "/Game/Magic___Spell_Sounds_PRO/General/cue/Magic_Explosion_2_Cue.Magic_Explosion_2_Cue" _returnvalue (struct) 1.0 1.0 0.0 null null null null))
    (:`then_2`
      (`SceneComponent.SetVisibility` (`self.Mesh`) false true)
      (cast `/Game/TalesContent/Blueprints/Ai/BP_CombatAi` (`AIBlueprintHelperLibrary.GetAIController` self))
      (`self.DetachFromControllerPendingDestroy`))))

(fn `UserConstructionScript`)