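; NPC_Skeleton is a skeleton NPC Blueprint that extends its parent's death handling with a bone-scatter effect.
; On CharacterDeath it runs the parent logic, then immediately activates death audio and a Niagara effect.
; After a brief delay it hides the mesh, and only the authority spawns a BP_Bone_Ejector with a limited bone lifetime at the actor's location.
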(event `self.CharacterDeath`
  (`parent.CharacterDeath`)
  (`|ExecutionSequence`
    (:`then_0`
      (`ActorComponent.Activate` (`self.DeathAudio`) true)
      (`ActorComponent.Activate` (`self.Niagara_Death_1`) true))
    (:`then_1`
      (`KismetSystemLibrary.Delay` 0.2)
      (`SceneComponent.SetVisibility` (`self.Mesh`) false false)
      (`/Engine/EditorBlueprintResources/ActorMacros.Switch Has Authority`
        (:`Authority`
          (`|SpawnActorFromClass` :`Class` "/Game/TalesContent/Blueprints/Effects/BP_Bone_Ejector.BP_Bone_Ejector_C" :`SpawnTransform` (`KismetMathLibrary.MakeTransform` (`self.K2_GetActorLocation`)) :`CollisionHandlingOverride` "AlwaysSpawn" :`TransformScaleMethod` "MultiplyWithRoot" :`BoneLifetime` 5.0 :`Instigator` null))))))

(fn `UserConstructionScript`
  (`parent.UserConstructionScript`))