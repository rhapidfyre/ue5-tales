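; Base Blueprint for combat NPCs that adds an overhead data widget to the character.
; On BeginPlay it links the widget to the character and positions it just above the top of the capsule.
; A looping timer, rather than Tick, rotates the widget to face the player camera and clears itself once the widget is invalid.
; On character death it destroys the widget component after calling the parent logic.
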(event `self.ReceiveBeginPlay`
  (bind _widget (`self.Widget`))
  (`parent.ReceiveBeginPlay`)
  (`|ExecutionSequence`
    (:`then_0`
      (bind _aswidget_overhead_player_data (cast `/Game/TalesContent/Widgets/Targeting/Widget_Overhead_PlayerData` (`WidgetComponent.GetWidget` _widget)))
      (`/Game/TalesContent/Widgets/Targeting/Widget_Overhead_PlayerData.SetCharacterReference` _aswidget_overhead_player_data self)
      (`SceneComponent.K2_SetWorldLocation` _widget (+ (`KismetMathLibrary.MakeVector` 0.0 0.0 (+ (`CapsuleComponent.CapsuleHalfHeight` (`self.CapsuleComponent`)) 20.0)) (`SceneComponent.K2_GetComponentLocation` (`self.CapsuleComponent`))) false true))
    (:`then_1`
      (bind _returnvalue (`KismetSystemLibrary.K2_SetTimerDelegate` (delegate `UpdateOverheadData_Timer`) 0.1 true))
      (set `self.OverheadTimer` _returnvalue))))

(event `UpdateOverheadData_Timer`
  (bind _returnvalue (`GameplayStatics.GetPlayerCameraManager` 0))
  (bind _widget (`self.Widget`))
  (`self.Widget`
    (:`then`
      (`/Engine/EditorBlueprintResources/StandardMacros.IsValid` _returnvalue
        (:`Is Valid`
          (`SceneComponent.K2_SetWorldRotation` _widget (`KismetMathLibrary.FindLookAtRotation` (`SceneComponent.K2_GetComponentLocation` _widget) (`self.K2_GetActorLocation` _returnvalue)) false false))))
    (:`else`
      (`KismetSystemLibrary.K2_ClearAndInvalidateTimerHandle` (`self.OverheadTimer`)))))

(event `self.CharacterDeath`
  (`parent.CharacterDeath`)
  (bind _widget (`self.Widget`)
    (:`then`
      (`ActorComponent.K2_DestroyComponent` _widget))
    (:`else`)))

(fn `UserConstructionScript`)