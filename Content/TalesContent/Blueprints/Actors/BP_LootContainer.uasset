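; Lootable container actor that plays open and close sounds through MC effect events and can award random currency to a character.
; Construction derives per-denomination reward ranges and caps at 70% of each range above the minimum.
; GetOpenReward rolls an overall chance, then scales each denomination by its own roll and chance, clamped to those caps.
; CheckForOpenReward adds the result to the character's InventoryComponent only while TimesOpened is below one.
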(event `MC_CloseEffects`
  (`AudioComponent.Play` (`self.AudioClose`) 0.0))

(event `MC_OpenEffects`
  (`AudioComponent.Play` (`self.AudioOpen`) 0.0))

(event `OpenContainer`
  (params (CharacterRef :type "CharacterBase Object Reference"))
  (`self.MC_OpenEffects`))

(event `CloseContainer`
  (`self.MC_CloseEffects`))

(event `/T5GInventorySystem/Game/InteractionInterface.StartInteraction`)

(fn `CheckForOpenReward`
  (params (OpeningCharacter :type "CharacterBase Object Reference"))
  (locals (tOpenReward :type "CurrencyData Structure"))
  (if (and (< (`self.TimesOpened`) 1) (`KismetSystemLibrary.IsValid` OpeningCharacter))
    (bind _openreward (`self.GetOpenReward`))
    (bind _output_get (set `local.tOpenReward` _openreward))
    (`InventoryComponent.AddCurrency` (`CharacterBase.InventoryComponent` OpeningCharacter) (`.Copper` (break `CurrencyData` _output_get)) (`.Silver` (break `CurrencyData` _output_get)) (`.Gold` (break `CurrencyData` _output_get)) (break `CurrencyData` _output_get))))

(fn `CheckInteractive`
  (returns (AboutObject :type "Object Object Reference"))
  (return self))

(fn `GetOpenReward`
  (returns (OpenReward :type "CurrencyData Structure"))
  (locals (tRollPlatinum :type "Float (double-precision)" :default 0.0) (tRollGold :type "Float (double-precision)" :default 0.0) (tRollSilver :type "Float (double-precision)" :default 0.0) (tRollCopper :type "Float (double-precision)" :default 0.0) (tReward :type "CurrencyData Structure") (tRewardPlatinum :type Integer) (tRewardGold :type Integer) (tRewardSilver :type Integer) (tRewardCopper :type Integer))
  (bind _chanceplat (`self.ChancePlat`))
  (bind (_rewardrange_platinum _rewardrange_gold _rewardrange_silver _rewardrange_copper) (break `CurrencyData` (`self.RewardRange`)))
  (bind (_randomawardmin_platinum _randomawardmin_gold _randomawardmin_silver _randomawardmin_copper) (break `CurrencyData` (`self.RandomAwardMin`)))
  (bind (_truereward_platinum _truereward_gold _truereward_silver _truereward_copper) (break `CurrencyData` (`self.TrueReward`)))
  (if (< (`self.ChanceOfReward`) (`KismetMathLibrary.RandomFloatInRange` 0.0 1.0))
    (`|ExecutionSequence`
      (:`then_0`
        (set `local.tRollPlatinum` (`KismetMathLibrary.RandomFloatInRange` 0.0 1.0))
        (set `local.tRollGold` (`KismetMathLibrary.RandomFloatInRange` 0.0 1.0))
        (set `local.tRollSilver` (`KismetMathLibrary.RandomFloatInRange` 0.0 1.0))
        (set `local.tRollCopper` (`KismetMathLibrary.RandomFloatInRange` 0.0 1.0)))
      (:`then_1`
        (set `local.tRewardPlatinum` (`KismetMathLibrary.Min` (+ (`KismetMathLibrary.Round` (* (`KismetMathLibrary.Conv_IntToDouble` _rewardrange_platinum) (- 1.0 (/ (- _chanceplat (`local.tRollPlatinum`)) _chanceplat)))) _randomawardmin_platinum) _truereward_platinum))
        (set `local.tRewardGold` (`KismetMathLibrary.SelectInt` (`KismetMathLibrary.Min` (+ (`KismetMathLibrary.Round` (* (`KismetMathLibrary.Conv_IntToDouble` _rewardrange_gold) (- 1.0 (/ (- (`self.ChanceGold`) (`local.tRollGold`)) 0.0)))) _randomawardmin_gold) _truereward_gold) 0 (< (`self.ChanceGold`) (`local.tRollGold`))))
        (set `local.tRewardSilver` (`KismetMathLibrary.SelectInt` (`KismetMathLibrary.Min` (+ (`KismetMathLibrary.Round` (* (`KismetMathLibrary.Conv_IntToDouble` _rewardrange_silver) (- 1.0 (/ (- (`self.ChanceSilver`) (`local.tRollSilver`)) 0.0)))) _randomawardmin_silver) _truereward_silver) 0 (< (`self.ChanceSilver`) (`local.tRollSilver`))))
        (set `local.tRewardCopper` (`KismetMathLibrary.SelectInt` (`KismetMathLibrary.Min` (+ (`KismetMathLibrary.Round` (* (`KismetMathLibrary.Conv_IntToDouble` _rewardrange_copper) (- 1.0 (/ (- (`self.ChanceCopper`) (`local.tRollCopper`)) 0.0)))) _randomawardmin_copper) _truereward_copper) 0 (< (`self.ChanceCopper`) (`local.tRollCopper`)))))
      (:`then_2`
        (return (make `CurrencyData` (`local.tRewardPlatinum`) (`local.tRewardGold`) (`local.tRewardSilver`) (`local.tRewardCopper`)))))
    (else
      (return (make `CurrencyData` 0)))))

(fn `UserConstructionScript`
  (bind (_randomawardmin_platinum _randomawardmin_gold _randomawardmin_silver _randomawardmin_copper) (break `CurrencyData` (`self.RandomAwardMin`)))
  (bind (_randomawardmax_platinum _randomawardmax_gold _randomawardmax_silver _randomawardmax_copper) (break `CurrencyData` (`self.RandomAwardMax`)))
  (`parent.UserConstructionScript`)
  (bind _output_get (set `self.RewardRange` (make `CurrencyData` (`KismetMathLibrary.Abs_Int` (- _randomawardmax_platinum _randomawardmin_platinum)) (`KismetMathLibrary.Abs_Int` (- _randomawardmax_gold _randomawardmin_gold)) (`KismetMathLibrary.Abs_Int` (- _randomawardmax_silver _randomawardmin_silver)) (`KismetMathLibrary.Abs_Int` (- _randomawardmax_copper _randomawardmin_copper)))))
  (bind (_platinum _gold _silver _copper) (break `CurrencyData` _output_get))
  (set `self.TrueReward` (make `CurrencyData` (+ (`KismetMathLibrary.Round` (* (`KismetMathLibrary.Conv_IntToDouble` _platinum) 0.7)) _randomawardmin_platinum) (+ (`KismetMathLibrary.Round` (* (`KismetMathLibrary.Conv_IntToDouble` _gold) 0.7)) _randomawardmin_gold) (+ (`KismetMathLibrary.Round` (* (`KismetMathLibrary.Conv_IntToDouble` _silver) 0.7)) _randomawardmin_silver) (+ (`KismetMathLibrary.Round` (* (`KismetMathLibrary.Conv_IntToDouble` _copper) 0.7)) _randomawardmin_copper))))