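; Dungeon entrance actor: a portal pedestal with a levitating book that sends overlapping players through via their BP_PlayerController's EnterRealmPortal.
; Timers stage the start, activate, idle and ready effects; the teleport detector's collision turns on at ready and off on close.
; Self-restarting timelines pulse pedestal lights by portal state and drift the book between levitation targets until it settles back.
; SetDungeonEntrance stores the dungeon spawn transform.
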(event `PortalFx_PedestalGlow`
  (bind _vfxglowintensityidle (`self.VfxGlowIntensityIdle`))
  (bind _islevitating (`self.IsLevitating`))
  (bind (_direction _newtrack_0) (`Timeline|Timeline` :!via `PlayFromStart`)
    (:`Update`
      (`LightComponent.SetIntensity` (`self.RectLight1`) (* _newtrack_0 (`KismetMathLibrary.SelectFloat` (`KismetMathLibrary.SelectFloat` 0.0 (`self.VfxGlowIntensityTemp`) (`self.IsPortalIdle`)) (`self.VfxGlowIntensityIdle`) _islevitating)))
      (`LightComponent.SetIntensity` (`self.RectLight2`) (* _newtrack_0 (`KismetMathLibrary.SelectFloat` (`KismetMathLibrary.SelectFloat` 0.0 (`self.VfxGlowIntensityTemp`) (`self.IsPortalIdle`)) (`self.VfxGlowIntensityIdle`) _islevitating)))
      (`LightComponent.SetIntensity` (`self.RectLight3`) (* _newtrack_0 (`KismetMathLibrary.SelectFloat` (`KismetMathLibrary.SelectFloat` 0.0 (`self.VfxGlowIntensityTemp`) (`self.IsPortalIdle`)) (`self.VfxGlowIntensityIdle`) _islevitating)))
      (`LightComponent.SetIntensity` (`self.RectLight4`) (* _newtrack_0 (`KismetMathLibrary.SelectFloat` (`KismetMathLibrary.SelectFloat` 0.0 (`self.VfxGlowIntensityTemp`) (`self.IsPortalIdle`)) (`self.VfxGlowIntensityIdle`) _islevitating)))
      (`LightComponent.SetIntensity` (`self.PointLight2`) (* _newtrack_0 (`KismetMathLibrary.SelectFloat` (* _vfxglowintensityidle 2.0) _vfxglowintensityidle _islevitating)))
      (`LightComponent.SetIntensity` (`self.PointLight3`) (* _newtrack_0 (`KismetMathLibrary.SelectFloat` (* _vfxglowintensityidle 2.0) _vfxglowintensityidle _islevitating)))
      (`LightComponent.SetIntensity` (`self.PointLight1`) (* _newtrack_0 (`KismetMathLibrary.SelectFloat` (* _vfxglowintensityidle 2.0) _vfxglowintensityidle _islevitating)))
      (`LightComponent.SetIntensity` (`self.PointLight`) (* _newtrack_0 (`KismetMathLibrary.SelectFloat` (* _vfxglowintensityidle 2.0) _vfxglowintensityidle _islevitating))))
    (:`Finished`
      (`self.PortalFx_PedestalGlow`))))

(event `self.ReceiveBeginPlay`
  (`parent.ReceiveBeginPlay`)
  (`|ExecutionSequence`
    (:`then_0`
      (`KismetSystemLibrary.K2_SetTimerDelegate` (delegate `PortalFx_PedestalGlow`) 0.1))))

(event `StartPortalEffects`
  (`|ExecutionSequence`
    (:`then_0`
      (`ActorComponent.Activate` (`self.FxPortalStart`) true)
      (`ActorComponent.Activate` (`self.SfxPortalBookStart`) true)
      (`KismetSystemLibrary.Delay` 0.2))
    (:`then_1`
      (set `self.IsLevitating` true)
      (set `self.VfxGlowIntensityTemp` (`self.VfxGlowIntensityStart`))
      (`KismetSystemLibrary.K2_SetTimerDelegate` (delegate `PortalFx_StartLevitation`) 0.05)
      (`KismetSystemLibrary.Delay` 1.2)
      (set `self.VfxGlowIntensityTemp` (`self.VfxGlowIntensityActive`)))))

(event `ClosePortal`
  (`ActorComponent.Deactivate` (`self.FxPortalReady`))
  (`ActorComponent.Deactivate` (`self.FxPortalStart`))
  (`ActorComponent.Deactivate` (`self.FxPortalIdle`))
  (`ActorComponent.Deactivate` (`self.FxPortalActive`))
  (`ActorComponent.Deactivate` (`self.SfxPortalBookStart`))
  (`ActorComponent.Deactivate` (`self.SfxPortalBookIdle`))
  (`ActorComponent.Deactivate` (`self.SfxPortalIdle`))
  (`ActorComponent.Activate` (`self.SfxPortalBookStop`) true)
  (set `self.IsPortalActivated` false)
  (set `self.IsPortalIdle` false)
  (`self.StopLevitation`)
  (`PrimitiveComponent.SetCollisionEnabled` (`self.TeleportDetector`) "NoCollision"))

(event `PortalFx_StartLevitation`
  (bind (_direction _newtrack_0) (`Timeline|Book_StartLevitation` :!via `PlayFromStart`)
    (:`Update`
      (`self.SetBookLevitationData` _newtrack_0))
    (:`Finished`
      (`self.BookLevitation`))))

(event `CreatePortal`
  ;[0.1 0.1 0.1 0.4 14] Use timers so that each event can be tweaked (Timers auto destroy when the event fires and isn't looped)
  (set `self.IsPortalIdle` true)
  (`self.PortalFx_Activate`)
  (`KismetSystemLibrary.K2_SetTimerDelegate` (`|CreateDelegate` :!event `PortalFx_Ready`) 1.0)
  (`KismetSystemLibrary.K2_SetTimerDelegate` (`|CreateDelegate` :!event `PortalFx_Idle`) 2.4))

(event `BookLevitation`
  (bind (_nextvector _nextrotation) (`self.GetNextLeviData`))
  (if (`self.IsLevitating`)
    (`|ExecutionSequence`
      (:`then_0`
        (set `self.LeviNextVector` _nextvector))
      (:`then_1`
        (set `self.LeviNextRotation` _nextrotation))
      (:`then_2`
        (bind (_direction _newtrack_0) (`Timeline|Book_IdleLevitation` :!via `PlayFromStart`)
          (:`Update`
            (`self.SetNextLevitationData` _newtrack_0))
          (:`Finished`
            (`self.BookLevitation`)))))
    (else
      (bind (_direction_2 _newtrack_0_2) (`Timeline|Book_StopLevitation` :!via `PlayFromStart`)
        (:`Update`
          (`self.SetBookLevitationData` _newtrack_0_2))))))

(event `PortalFx_Ready`
  (`ActorComponent.Activate` (`self.FxPortalReady`) true)
  (`PrimitiveComponent.SetCollisionEnabled` (`self.TeleportDetector`) "QueryOnly"))

(event `PortalFx_Idle`
  (`ActorComponent.Activate` (`self.FxPortalIdle`) true)
  (`ActorComponent.Activate` (`self.SfxPortalIdle`) true))

(event `StopLevitation`
  (set `self.IsLevitating` false))

(event `self.TeleportDetector.OnComponentBeginOverlap`
  (params (OverlappedComponent :type "PrimitiveComponent Object Reference") (OtherActor :type "Actor Object Reference") (OtherComp :type "PrimitiveComponent Object Reference") (OtherBodyIndex :type Integer) (bFromSweep :type Boolean) (SweepResult :type "HitResult Structure (by ref)"))
  (`KismetSystemLibrary.PrintString` (`KismetStringLibrary.Concat_StrStr` "Overlapped by " (`KismetSystemLibrary.GetDisplayName` OtherActor)))
  (bind _asbp_player_controller (cast `/Game/TalesContent/Gamemode/BP_PlayerController` (`self.GetInstigatorController` OtherActor)))
  (`/Game/TalesContent/Gamemode/BP_PlayerController.EnterRealmPortal` _asbp_player_controller))

(event `PortalFx_Activate`
  (`ActorComponent.Activate` (`self.FxPortalActive`) true)
  (`ActorComponent.Deactivate` (`self.FxPortalStart`))
  (`ActorComponent.Activate` (`self.SfxPortalBookIdle`) true)
  (`ActorComponent.Deactivate` (`self.SfxPortalBookStart`))
  (set `self.IsPortalActivated` true))

(fn `CheckInteractive`
  (returns (AboutObject :type "Object Object Reference"))
  (return self))

(fn `SetBookLevitationData`
  (params (Delta :type "Float (single-precision)"))
  (`SceneComponent.K2_SetRelativeLocationAndRotation` (`self.SM_Prop_Book_Open_02`) (`KismetMathLibrary.VLerp` (`self.OriginPoint`) (`self.BookVector`) Delta) (`KismetMathLibrary.RLerp` (`self.OriginRotation`) (`self.BookRotation`) Delta true) false false))

(fn `SetDungeonEntrance`
  (params (InSpawnData :type "Transform Structure"))
  (set `self.DungeonSpawn` (`KismetMathLibrary.MakeTransform` (.location InSpawnData) (.rotation InSpawnData))))

(fn `SetNextLevitationData`
  (params (Alpha :type "Float (single-precision)"))
  (`SceneComponent.K2_SetRelativeLocationAndRotation` (`self.SM_Prop_Book_Open_02`) (`KismetMathLibrary.VLerp` (`self.BookVector`) (`self.LeviNextVector`) Alpha) (`KismetMathLibrary.RLerp` (`self.BookRotation`) (`self.LeviNextRotation`) Alpha true) false false))

(fn `UserConstructionScript`
  (`parent.UserConstructionScript`)
  (`FXSystemComponent.SetVectorParameter` (`self.FxPortalActive`) "color" (`KismetMathLibrary.Conv_LinearColorToVector` (`self.FxColor`)))
  (`SceneComponent.K2_SetRelativeTransform` (`self.SM_Prop_Book_Open_02`) (`KismetMathLibrary.MakeTransform` (`self.OriginPoint`) (`self.OriginRotation`) (1.35 1.35 1.0)) false true)
  (`LightComponent.SetIntensity` (`self.RectLight1`) (`self.VfxGlowIntensityIdle`))
  (`LightComponent.SetIntensity` (`self.RectLight2`) (`self.VfxGlowIntensityIdle`))
  (`LightComponent.SetIntensity` (`self.RectLight3`) (`self.VfxGlowIntensityIdle`))
  (`LightComponent.SetIntensity` (`self.RectLight4`) (`self.VfxGlowIntensityIdle`)))