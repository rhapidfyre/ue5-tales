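; Homing spell projectile that chases a target actor and sets it ablaze when it gets close.
; On authority, each tick turns it toward a valid target and drives ProjectileMovement velocity along its forward vector.
; Proximity is a distance check: within range it destroys itself and applies GE_Ablaze, using a spec made by the target's own Ability System Component.
; The Niagara asset setup and movement activation nodes are unconnected.
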(event `self.ReceiveBeginPlay`
  (`parent.ReceiveBeginPlay`)
  (set `self.OriginVector` (`self.K2_GetActorLocation`)))

(event `self.ReceiveTick`
  (params (DeltaSeconds :type "Float (single-precision)"))
  (`parent.ReceiveTick` DeltaSeconds)
  (`/Engine/EditorBlueprintResources/ActorMacros.Switch Has Authority`
    (:`Authority`
      (`self.UpdateProjectile`))))

(fn `UpdateProjectile`
  (bind _returnvalue (`AbilitySystemBlueprintLibrary.GetAbilitySystemComponent` (`self.TargetActor`)))
  (`|ExecutionSequence`
    (:`then_1`
      (bind _targetactor (`self.TargetActor`)
        (:`then`
          (`|ExecutionSequence`
            (:`then_0`
              (if (< (`KismetMathLibrary.Vector_Distance` (`self.K2_GetActorLocation`) (`self.K2_GetActorLocation` _targetactor)) 100.0)
                (`self.SetActorTickEnabled` false)
                (`self.K2_DestroyActor`)
                (`AbilitySystemComponent.BP_ApplyGameplayEffectSpecToSelf` _returnvalue (`AbilitySystemComponent.MakeOutgoingSpec` :`self` _returnvalue :`GameplayEffectClass` "/RoleStats/Effects/Testing/GE_Ablaze.GE_Ablaze_C"))
                (return)))
            (:`then_1`
              (`self.K2_SetActorRotation` (`KismetMathLibrary.FindLookAtRotation` (`self.K2_GetActorLocation`) (`self.K2_GetActorLocation` _targetactor))))))
        (:`else`)))
    (:`then_2`
      (set `MovementComponent.Velocity` (* (`self.GetActorForwardVector`) (`self.ProjectileSpeed`)) (`self.ProjectileMovement`)))))

(fn `UserConstructionScript`)