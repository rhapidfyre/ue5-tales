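; BP_LootBox_Tomb_1 is a tomb loot box variant that adds an animated lid to its parent's open and close effects.
; The construction script stores the lid's placed rotation as the closed pose.
; MCOpenEffects plays a timeline that lerps the lid's roll from that pose by the FullyOpenRotation offset.
; MCCloseEffects reverses the same timeline from the end to shut it.
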(event `self.MC_OpenEffects`
  (bind (_closedrotation_roll _closedrotation_pitch _closedrotation_yaw) (`KismetMathLibrary.BreakRotator` (`self.ClosedRotation`)))
  (`parent.MC_OpenEffects`)
  (bind (_direction _newtrack_0) (`Timeline|Timeline_ChestLid` :!via `PlayFromStart` :!label _label)
    (:`Update`
      (`SceneComponent.K2_SetRelativeRotation` (`self.ChestLid`) (`KismetMathLibrary.RLerp` (`self.ClosedRotation`) (`KismetMathLibrary.MakeRotator` (+ _closedrotation_roll (`self.FullyOpenRotation`)) _closedrotation_pitch _closedrotation_yaw) _newtrack_0) false false))))

(event `self.MC_CloseEffects`
  (`parent.MC_CloseEffects`)
  (goto _label :!via `ReverseFromEnd`))

(fn `UserConstructionScript`
  (`parent.UserConstructionScript`)
  (set `self.ClosedRotation` (`SceneComponent.RelativeRotation` (`self.ChestLid`))))