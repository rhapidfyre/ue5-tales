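; BP_Trap_Wet is a trap that applies a gameplay effect, presumably a wet status, to characters within its Box volume.
; On actor overlap it runs the parent logic, then, on authority only, gathers every CharacterBase inside the box rather than just the entering actor.
; Each character's ability system component builds a spec from OnPickupEffect and applies it to itself, so the trap is not the effect's source.
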(event `self.ReceiveActorBeginOverlap`
  (params (OtherActor :type "Actor Object Reference"))
  (`parent.ReceiveActorBeginOverlap` OtherActor)
  (`/Engine/EditorBlueprintResources/ActorMacros.Switch Has Authority`
    (:`Authority`
      (for _array_element (`PrimitiveComponent.GetOverlappingActors` (`self.Box`) "/Script/TalesDungeoneer.CharacterBase")
        (bind _ascharacter_base (cast `CharacterBase` _array_element))
        (bind _returnvalue (`AbilitySystemBlueprintLibrary.GetAbilitySystemComponent` _ascharacter_base))
        (if (`KismetSystemLibrary.IsValid` _returnvalue)
          (`AbilitySystemComponent.BP_ApplyGameplayEffectSpecToSelf` _returnvalue (`AbilitySystemComponent.MakeOutgoingSpec` _returnvalue (`self.OnPickupEffect`) 1.0 (`AbilitySystemComponent.MakeEffectContext` _returnvalue))))))))

(fn `UserConstructionScript`)