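; Template gameplay ability for a melee weapon attack that damages characters caught in the owner's strike detector.
; After committing, it waits for the hit-detect delay, then samples the detector's overlaps once, skipping the owner.
; Each target with an ability system receives the melee damage effect at the attacker's level, with negated base damage passed via SetByCaller.
; The ability stays active for the remaining cooldown time before ending.
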(event `self.K2_ActivateAbility`
  (`parent.K2_ActivateAbility`)
  (cast `CharacterBase` (`self.GetAvatarActorFromActorInfo`)
    (:`then`
      (bind _returnvalue (`self.K2_CommitAbility`))
      (if _returnvalue
        (`KismetSystemLibrary.Delay` (`self.DelayHitDetect`))
        (bind _ascharacter_base (cast `CharacterBase` (`self.GetAvatarActorFromActorInfo`)))
        (for _array_element (`PrimitiveComponent.GetOverlappingActors` (`CharacterBase.MeleeStrikeDetector` _ascharacter_base) "/Script/TalesDungeoneer.CharacterBase")
          (if (!= _array_element _ascharacter_base)
            (bind _returnvalue_2 (`AbilitySystemBlueprintLibrary.GetAbilitySystemComponent` _array_element))
            (if (`KismetSystemLibrary.IsValid` _returnvalue_2)
              (bind _returnvalue_3 (`AbilitySystemBlueprintLibrary.GetAbilitySystemComponent` _ascharacter_base))
              (bind _returnvalue_4 (`AbilitySystemBlueprintLibrary.AssignTagSetByCallerMagnitude` (`AbilitySystemComponent.MakeOutgoingSpec` _returnvalue_3 "/RoleStats/Effects/GE_Damage_Melee_Base.GE_Damage_Melee_Base_C" (`KismetMathLibrary.Conv_IntToDouble` (`CharacterBase.GetCharacterLevel` _ascharacter_base)) (`AbilitySystemComponent.MakeEffectContext` _returnvalue_2)) (struct :`TagName` "Damage.SetByCaller") (* (`self.AttackDamageBase`) -1.0)))
              (`AbilitySystemComponent.BP_ApplyGameplayEffectSpecToTarget` _returnvalue_3 _returnvalue_4 _returnvalue_2))))
        (`KismetSystemLibrary.Delay` (- (`self.CooldownTime`) (`self.DelayHitDetect`)))
        (`self.K2_EndAbility`)
        (else
          (`self.K2_EndAbility`))))
    (:`CastFailed`
      (`self.K2_EndAbility`))))