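; Gameplay ability for a Firebolt spell that plays a slowed cast montage and launches a fire projectile.
; During the cast, the server attaches a casting effect actor to the right hand.
; On blend out, interrupt or cancel, it destroys that actor and fires BP_Projectile_Spell from the hand at the first CombatNpcCharacterBase found in the world.
; The ability ends only on montage completion.
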(event `self.K2_ActivateAbility`
  (bind _returnvalue (`self.GetAvatarActorFromActorInfo`))
  (bind _projectileref (`self.ProjectileRef`))
  (`|ExecutionSequence`
    (:`then_0`
      (`self.K2_CommitAbility`))
    (:`then_1`
      (`AbilityTask_PlayMontageAndWait.CreatePlayMontageAndWaitProxy` "None" "/Game/Blink/Characters/LowPoly/Humans/Male/Anims/Anim_SpellCast_Montage.Anim_SpellCast_Montage" 0.4
        (:`then`
          (`self.K2_HasAuthority`
            (:`True`
              (bind _ascharacter_base (cast `CharacterBase` (`self.GetAvatarActorFromActorInfo`)))
              (bind _mesh (`Character.Mesh` _ascharacter_base))
              (bind _returnvalue_2 (`|SpawnActorFromClass` "/Game/TalesContent/Blueprints/Actors/Spells/BP_Casting_Fire.BP_Casting_Fire_C" (`KismetMathLibrary.MakeTransform` (`SceneComponent.GetSocketLocation` _mesh "hand_r")) "Undefined" "MultiplyWithRoot" null null))
              (bind _output_get (set `self.ProjectileRef` _returnvalue_2))
              (`Actor.K2_AttachToComponent` _output_get _mesh "hand_r" "SnapToTarget" "SnapToTarget" "SnapToTarget" true))))
        (:`OnCompleted`
          (`self.K2_EndAbility`))
        (:`OnBlendOut`
          (`|ExecutionSequence` :!label _label
            (:`then_0`
              (`self.K2_HasAuthority`
                (:`True`
                  (`/Engine/EditorBlueprintResources/StandardMacros.IsValid` _projectileref
                    (:`Is Valid`
                      (`Actor.K2_DestroyActor` _projectileref))))))
            (:`then_1`
              (`self.K2_HasAuthority`
                (:`True`
                  (bind _ascharacter_base_2 (cast `CharacterBase` _returnvalue))
                  (bind _outactors (`GameplayStatics.GetAllActorsOfClass` "/Script/TalesDungeoneer.CombatNpcCharacterBase"))
                  (bind _returnvalue_3 (`SceneComponent.GetSocketLocation` (`Character.Mesh` _ascharacter_base_2) "hand_r"))
                  (bind _output (`|GetArrayItem` _outactors))
                  (`|SpawnActorFromClass` "/Game/TalesContent/Blueprints/Actors/Projectiles/BP_Projectile_Spell.BP_Projectile_Spell_C" (`KismetMathLibrary.MakeTransform` _returnvalue_3 (`KismetMathLibrary.FindLookAtRotation` _returnvalue_3 (`Actor.K2_GetActorLocation` _output))) "AlwaysSpawn" "MultiplyWithRoot" null "/Game/Magic_Projectiles/MagicProjectiles/Niagara/Fire/NS_Fire_Trail.NS_Fire_Trail" _returnvalue _output 1200.0 null))))))
        (:`OnInterrupted`
          (goto _label))
        (:`OnCancelled`
          (goto _label))))))