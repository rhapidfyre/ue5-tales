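; Player controller for the Tales game, handling menu and inventory input, interaction, death screen and environment music.
; Interact dispatches by target type to HUD windows for NPCs, loot and dungeon generation, or to leaving a dungeon.
; Server events relay dungeon, portal and loot-closing requests to game state and actors.
; A one-second timer drives music, fading in queued tracks at saved times or random idle tracks when the queue is empty.
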(event `InitCharacterRef`
  (bind _ascharacter_base (cast `CharacterBase` (`self.K2_GetPawn`))
    (:`then`
      (bind _output_get (set `self.CharacterRef` _ascharacter_base))
      (add `RsAbilityComponent.OnDeathStatusChanged` (`CharacterBase.AbilitySystemComponent` _output_get) (`|CreateDelegate` :!event `Callback_OnDeathStatus`)))
    (:`CastFailed`
      (`KismetSystemLibrary.Delay` 0.2)
      (`self.InitCharacterRef`))))

(event `self.ReceiveBeginPlay`
  (`parent.ReceiveBeginPlay`)
  (`|ExecutionSequence`
    (:`then_0`
      (`self.InitCharacterRef`))
    (:`then_1`
      (`KismetSystemLibrary.K2_SetTimerDelegate` (delegate `Timer_MusicQueue`) 1.0 true))))

(event `self.ReceiveTick`
  (params (DeltaSeconds :type "Float (single-precision)"))
  (bind _currenttracktime (`self.CurrentTrackTime`))
  (`parent.ReceiveTick` DeltaSeconds)
  (`self.CurrentMusicTrack`
    (:`then`
      (set `self.CurrentTrackTime` (+ _currenttracktime DeltaSeconds)))
    (:`else`
      (if (not (`KismetMathLibrary.NearlyEqual_FloatFloat` _currenttracktime 0.0 0.001))
        (set `self.CurrentTrackTime` 0.0)))))

(event `Timer_MusicQueue`
  (`/Engine/EditorBlueprintResources/StandardMacros.IsValid` (`self.CurrentMusicTrack`)
    (:`Is Valid`
      (bind _audiocomponent (`self.AudioComponent`)
        (:`then`
          (if (not (`AudioComponent.IsPlaying` _audiocomponent))
            (`self.EnvMusicNext`)))
        (:`else`)))
    (:`Is Not Valid`
      (`self.EnvMusicNext`))))

(event `EnhancedInput|/Game/TalesContent/Inputs/Actions/IA_Menu_Key`
  (params (ActionValue :type Boolean) (ElapsedSeconds :type "Float (double-precision)") (TriggeredSeconds :type "Float (double-precision)") (InputAction :type "InputAction Object Reference" :default "/Game/TalesContent/Inputs/Actions/IA_Menu_Key.IA_Menu_Key"))
  (:`Started`
    (bind _asbp_tales_hud (cast `/Game/TalesContent/Gamemode/BP_TalesHud` (`self.GetHUD`)))
    (if (> (`KismetArrayLibrary.Array_Length` (`/Game/TalesContent/Gamemode/BP_TalesHud.GetAllVisibleWidgets` _asbp_tales_hud true)) 0)
      (`/Game/TalesContent/Gamemode/BP_TalesHud.CloseWidget` _asbp_tales_hud false)
      (else
        (cast `CharacterBase` (`GameplayStatics.GetPlayerCharacter` 0)
          (:`then`
            (`/Engine/EditorBlueprintResources/StandardMacros.IsValid` null ; Is Targeted Actor Valid
              (:`Is Not Valid`
                _)))
          (:`CastFailed`
            _))
        (`/Game/TalesContent/Gamemode/BP_TalesHud.ToggleMainMenu` _asbp_tales_hud true false)))))

(event `EnhancedInput|/Game/TalesContent/Inputs/Actions/IA_Inventory_Key`
  (params (ActionValue :type Boolean) (ElapsedSeconds :type "Float (double-precision)") (TriggeredSeconds :type "Float (double-precision)") (InputAction :type "InputAction Object Reference" :default "/Game/TalesContent/Inputs/Actions/IA_Inventory_Key.IA_Inventory_Key"))
  (:`Started`
    (bind _asbp_tales_hud (cast `/Game/TalesContent/Gamemode/BP_TalesHud` (`self.GetHUD`)))
    (`/Game/TalesContent/Gamemode/BP_TalesHud.ToggleInventory` _asbp_tales_hud)))

(event `PrepareDungeon`
  (params (DungeonName :type Name))
  (`self.SV_PrepareDungeon` DungeonName))

(event `Callback_OnDeathStatus`
  (params (bIsNowDead :type Boolean) (CurrentHealth :type "Float (single-precision)"))
  (if bIsNowDead
    (if (`self.IsLocalPlayerController`)
      (bind _returnvalue (`|CreateWidget` "/Game/TalesContent/Widgets/HUD_Death.HUD_Death_C"))
      (set `self.DeathWidget` _returnvalue)
      (`UserWidget.AddToViewport` _returnvalue 0)
      (`WidgetBlueprintLibrary.SetInputMode_UIOnlyEx` self _returnvalue "DoNotLock" true))
    (else
      (`|ExecutionSequence`
        (:`then_0`
          (bind _deathwidget (`self.DeathWidget`)
            (:`then`
              (`Widget.RemoveFromParent` _deathwidget))
            (:`else`)))
        (:`then_1`
          (bind _asbp_tales_hud (cast `/Game/TalesContent/Gamemode/BP_TalesHud` (`self.GetHUD`)))
          (`/Game/TalesContent/Gamemode/BP_TalesHud.UpdateControlFocus` _asbp_tales_hud))))))

(event `CloseLootContainer`
  (params (InvReference :type "InventoryComponent Object Reference"))
  (`self.SV_CloseLootContainer` InvReference))

(event `SV_CloseLootContainer`
  (params (InputObject :type "InventoryComponent Object Reference"))
  (`/Engine/EditorBlueprintResources/StandardMacros.IsValid` InputObject
    (:`Is Valid`
      (bind _asbp_loot_container (cast `/Game/TalesContent/Blueprints/Actors/BP_LootContainer` (`ActorComponent.GetOwner` InputObject)))
      (`/Game/TalesContent/Blueprints/Actors/BP_LootContainer.CloseContainer` _asbp_loot_container))))

(event `SV_PrepareDungeon`
  (params (DungeonName :type Name))
  (bind _asbp_tales_game_state (cast `/Game/TalesContent/Gamemode/BP_TalesGameState` (`GameplayStatics.GetGameState`)))
  (`/Game/TalesContent/Gamemode/BP_TalesGameState.GenerateDungeon` _asbp_tales_game_state DungeonName))

(event `EnhancedInput|/Game/TalesContent/Inputs/Actions/IA_Interact`
  (params (ActionValue :type Boolean) (ElapsedSeconds :type "Float (double-precision)") (TriggeredSeconds :type "Float (double-precision)") (InputAction :type "InputAction Object Reference" :default "/Game/TalesContent/Inputs/Actions/IA_Interact.IA_Interact"))
  (bind _returnvalue (`self.GetHUD`))
  (:`Started`
    (bind _astales_player (cast `/Game/TalesContent/Blueprints/Player/Tales_Player` (`self.CharacterRef`)))
    (bind _asactor (cast `Actor` (`/Game/TalesContent/Blueprints/Player/Tales_Player.GetInteractiveActor` _astales_player)))
    (`/Engine/EditorBlueprintResources/StandardMacros.IsValid` (`self.GetComponentByClass` _asactor "/Script/T5GInventorySystem.CraftingComponent") ; Crafting Station
      (:`Is Valid`
        (`KismetSystemLibrary.PrintString` "Crafting Not Yet Implemented")
        (cast `/Game/TalesContent/Gamemode/BP_TalesHud` (`self.GetHUD`)))
      (:`Is Not Valid`
        (bind _asinteractive_npc_character_base (cast `InteractiveNpcCharacterBase` _asactor)
          (:`then`
            (bind _asbp_tales_hud (cast `/Game/TalesContent/Gamemode/BP_TalesHud` _returnvalue))
            (`/Game/TalesContent/Gamemode/BP_TalesHud.StartNpcTransaction` _asbp_tales_hud _asinteractive_npc_character_base))
          (:`CastFailed`
            (bind _asbp_loot_container (cast `/Game/TalesContent/Blueprints/Actors/BP_LootContainer` _asactor)
              (:`then`
                (`/Game/TalesContent/Blueprints/Actors/BP_LootContainer.OpenContainer` _asbp_loot_container null)
                (bind _asbp_tales_hud_2 (cast `/Game/TalesContent/Gamemode/BP_TalesHud` _returnvalue))
                (`/Game/TalesContent/Gamemode/BP_TalesHud.OpenLootWindow` _asbp_tales_hud_2 (`/Game/TalesContent/Blueprints/Actors/BP_LootContainer.Inventory` _asbp_loot_container)))
              (:`CastFailed`
                (cast `/Game/TalesContent/Blueprints/Actors/BP_Dungeon_Entrance` _asactor
                  (:`then`
                    (bind _asbp_tales_hud_3 (cast `/Game/TalesContent/Gamemode/BP_TalesHud` (`self.GetHUD`)))
                    (`/Game/TalesContent/Gamemode/BP_TalesHud.OpenDungeonGen` _asbp_tales_hud_3))
                  (:`CastFailed`
                    (cast `/Game/TalesContent/Blueprints/Actors/BP_Dungeon_Exit` _asactor)
                    (`self.Server_LeaveDungeon`)))))))))))

(event `EnterRealmPortal`
  (`self.SV_EnterRealmPortal`))

(event `SV_EnterRealmPortal`
  (bind _asbp_tales_game_state (cast `/Game/TalesContent/Gamemode/BP_TalesGameState` (`GameplayStatics.GetGameState`)))
  (`/Game/TalesContent/Gamemode/BP_TalesGameState.SendPlayerToDungeon` _asbp_tales_game_state (`self.CharacterRef`)))

(event `QueueEnvMusic`
  (params (NextTrack :type "SoundBase Class Reference"))
  (`self.AudioComponent`
    (:`then`
      (if (`KismetSystemLibrary.IsValidClass` NextTrack) :!label _label
        (bind _returnvalue (`|GenericCreateObject` NextTrack))
        (`GameplayStatics.SpawnSound2D` _returnvalue 0.65 1.0 0.0 null true)))
    (:`else`
      (`|ExecutionSequence`
        (:`then_0`
          (bind _returnvalue_2 (`|AddComponentByClass` "/Script/Engine.AudioComponent" false (`KismetMathLibrary.MakeTransform` (0.0 0.0 0.0))))
          (set `self.AudioComponent` _returnvalue_2))
        (:`then_1`
          (goto _label))
        (:`then_2`
          (if (`BlueprintMapLibrary.Map_IsEmpty` (`self.MusicQueue`))
            _))))))

(event `Server_LeaveDungeon`
  (bind _returnvalue (`GameplayStatics.GetActorOfClass` "/Game/TalesContent/Blueprints/Actors/BP_Dungeon_Entrance.BP_Dungeon_Entrance_C"))
  (`/Engine/EditorBlueprintResources/StandardMacros.IsValid` _returnvalue
    (:`Is Valid`
      (bind _spawnpoint (`/Game/TalesContent/Blueprints/Actors/BP_Dungeon_Entrance.Spawnpoint` _returnvalue)
        (:`then`
          (bind (_returnvalue_location _returnvalue_rotation) (`KismetMathLibrary.BreakTransform` (`SceneComponent.K2_GetComponentToWorld` _spawnpoint)))
          (`self.K2_SetActorLocationAndRotation` (`self.K2_GetPawn`) _returnvalue_location _returnvalue_rotation false true))
        (:`else`
          (`self.K2_SetActorLocationAndRotation` :`self` (`self.K2_GetPawn`) :`bTeleport` true :!label _label_2))))
    (:`Is Not Valid`
      (goto _label_2))))

(event `EnvMusicTrack_FadeOut`
  (params (DelayTime :type "Float (double-precision)") (AutoPlayNext :type Boolean))
  (bind _audiocomponent (`self.AudioComponent`)
    (:`then`
      (`AudioComponent.FadeOut` _audiocomponent (`self.EnvMusicFadeOut`) 0.0 "Linear")
      (`KismetSystemLibrary.Delay` (+ DelayTime 0.01))
      (if AutoPlayNext
        (`self.EnvMusicNext`)))
    (:`else`
      (if AutoPlayNext
        (`self.EnvMusicNext`)))))

(fn `EnvMusicNext`
  (locals (tNextTrack :type "SoundBase Object Reference") (tStartTime :type "Float (double-precision)") (tSoundIndex :type Integer :default 0) (tSoundArray :type "Array of SoundBase Object Reference"))
  (bind _tsoundindex (`local.tSoundIndex`))
  (bind _musicqueue (`self.MusicQueue`))
  (bind _tstarttime (`local.tStartTime`))
  (bind _tsoundarray (`local.tSoundArray`))
  (bind (_value _returnvalue) (`BlueprintMapLibrary.Map_Find` (`self.MusicQueue`) (`local.tNextTrack`)))
  (bind (_value_2 _returnvalue_2) (`BlueprintMapLibrary.Map_Find` (`self.MusicQueue`) (`local.tNextTrack`)))
  (`|ExecutionSequence`
    (:`then_0`
      (if (`BlueprintMapLibrary.Map_IsEmpty` _musicqueue)
        ;[0.1 0.1 0.1 0.4] If queue is empty, select a random idle song
        (set `local.tNextTrack` (`KismetArrayLibrary.Array_Random` (`self.EnvMusicList`)))
        (else
          (bind _keys (`BlueprintMapLibrary.Map_Keys` _musicqueue))
          (bind _output_get (set `local.tSoundArray` _keys))
          (for _array_element _output_get
            ;[0.1 0.1 0.1 0.6] Resume any song that was interrupted
            (if _returnvalue_2
              (if (> _value_2 1.0)
                (set `local.tNextTrack` _array_element))))
          (if (`KismetArrayLibrary.Array_IsValidIndex` _tsoundarray _tsoundindex)
            (set `local.tNextTrack` (`|GetArrayItem` _tsoundarray _tsoundindex))
            (if _returnvalue
              (set `local.tStartTime` _value))))))
    (:`then_1`
      ;[0.1 0.1 0.1 0.4] Anything to play? If not, invalidate the timer for memory.
      (`local.tNextTrack`
        (:`then`
          (set `self.CurrentMusicTrack` (`local.tNextTrack`))
          (`|ExecutionSequence`
            (:`then_0`
              (`self.AudioComponent`
                (:`then`)
                (:`else`
                  (bind _returnvalue_3 (`AddComponent|NODE_AddAudioComponent-0`))
                  (set `self.AudioComponent` _returnvalue_3))))
            (:`then_1`
              (bind _audiocomponent (`self.AudioComponent`)
                (:`then`
                  (`AudioComponent.SetSound` _audiocomponent (`self.CurrentMusicTrack`))
                  (`AudioComponent.FadeIn` _audiocomponent (`self.EnvMusicFadeIn`) (`self.EnvMusicVolume`) _tstarttime "Linear")
                  (set `self.CurrentTrackTime` _tstarttime))
                (:`else`)))))
        (:`else`
          (`KismetSystemLibrary.K2_ClearAndInvalidateTimerHandle` (`self.MusicTimerHandle`))
          (`ActorComponent.K2_DestroyComponent` (`self.AudioComponent`))
          (set `self.CurrentMusicTrack` null))))))

(fn `EnvMusicPlayNow`
  (params (NextTrackRef :type "SoundBase Object Reference"))
  (`|ExecutionSequence`
    (:`then_0`
      (bind _currentmusictrack (`self.CurrentMusicTrack`)
        (:`then`
          (`BlueprintMapLibrary.Map_Add` (`self.MusicQueue`) _currentmusictrack (`self.CurrentTrackTime`)))
        (:`else`)))
    (:`then_2`
      (`/Engine/EditorBlueprintResources/StandardMacros.IsValid` NextTrackRef
        (:`Is Valid`
          (`self.EnvMusicTrack_FadeOut` 0.0)
          (`self.AudioComponent`
            (:`then`
              _)
            (:`else`
              (bind _returnvalue (`AddComponent|NODE_AddAudioComponent-1`))
              (set `self.AudioComponent` _returnvalue)))
          (bind _audiocomponent (`self.AudioComponent`)
            (:`then`
              (`AudioComponent.SetSound` _audiocomponent (`local.NextTrackRef`))
              (`AudioComponent.FadeIn` _audiocomponent (`self.EnvMusicFadeIn`) 1.0 0.0 "Linear"))
            (:`else`)))))))

(fn `PurchaseItem`
  (params (TargetInventory :type "InventoryComponent Object Reference") (SlotNumber :type Integer) (BuyPrice :type "Float (double-precision)")))

(fn `SellItem`
  (params (TargetInventory :type "InventoryComponent Object Reference") (SlotNumber :type Integer) (BuyPrice :type "Float (double-precision)"))
  (bind _returnvalue (`self.GetComponentByClass` (`GameplayStatics.GetPlayerCharacter` 0) "/Script/T5GInventorySystem.InventoryComponent"))
  (`InventoryComponent.Server_TransferItems` _returnvalue TargetInventory _returnvalue SlotNumber 0 1))

(fn `UserConstructionScript`)