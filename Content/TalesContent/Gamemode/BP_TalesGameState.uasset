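; Game state that runs procedural dungeon generation and connects its dungeon entrance portals.
; GenerateDungeon spawns a PCG tomb generator far below the world origin, with a random room count drawn from a data table row.
; A looping timer polls for completion, then readies portals on all entrances and passes them the dungeon transform.
; Helper functions expose the dungeon spawn point and teleport a player there; the portal-end event does nothing yet.
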(event Custom|MC_PortalEnd
  (bind _outactors (Actor|GetAllActorsOfClass "/Game/TalesContent/Blueprints/Actors/BP_Dungeon_Entrance.BP_Dungeon_Entrance_C"))
  (for _array_element _outactors
    _))

(event Custom|Timer_PcgCheck
  (bind _pcgactor (Variables|Default|GetPcgActor)
    (:then
      (if (Variables|/RealmsForge/ProcGen/BP_Rf_Dungeon_Generator.BP_Rf_Dungeon_Generator_C|GetGenerationComplete _pcgactor)
        (Utilities|FlowControl|Sequence
          (:then_0
            (Utilities|Time|ClearandInvalidateTimerbyHandle (Variables|Default|GetProcGenTimer) :!label _label))
          (:then_1
            (CallFunction|MCPortalReady)
            (bind _outactors (Actor|GetAllActorsOfClass "/Game/TalesContent/Blueprints/Actors/BP_Dungeon_Entrance.BP_Dungeon_Entrance_C"))
            (for _array_element _outactors
              (Default|SetDungeonEntrance _array_element (Transformation|GetActorTransform (Variables|Default|GetPcgActor))))))))
    (:else
      (goto _label))))

(event Custom|GenerateDungeon
  (params (PcgRowName :type Name))
  (CallFunction|MCPortalStart)
  (bind _returnvalue (Utilities|GetDataTableRow "/Game/TalesContent/DataTables/DT_DungeonGen.DT_DungeonGen" PcgRowName)
    (:then
      (bind _returnvalue_2 (Game|SpawnActorfromClass "/Game/TalesContent/Blueprints/PCG/Tomb/BP_PCG_Tomb_Gen.BP_PCG_Tomb_Gen_C" (Math|Transform|MakeTransform "0.000000,0.000000,-10000.000000" "0, 0, 0" "1.000000,1.000000,1.000000") "AlwaysSpawn" "MultiplyWithRoot" 0 0 (Math|Random|RandomIntegerinRange (.RoomsMinimum (Utilities|Struct|BreakST_DungeonGen _returnvalue)) (.RoomsMaximum (Utilities|Struct|BreakST_DungeonGen _returnvalue))) 0.05 0 100 0 0))
      (Variables|Default|SetPcgActor _returnvalue_2)
      (bind _returnvalue_3 (Utilities|Time|SetTimerbyEvent (delegate Custom|Timer_PcgCheck) 3.0 true false 1.0))
      (Variables|Default|SetProcGenTimer _returnvalue_3))))

(event Custom|MC_PortalStart
  (bind _outactors (Actor|GetAllActorsOfClass "/Game/TalesContent/Blueprints/Actors/BP_Dungeon_Entrance.BP_Dungeon_Entrance_C"))
  (for _array_element _outactors
    (Default|StartPortalEffects _array_element)))

(event Custom|MC_PortalReady
  (bind _outactors (Actor|GetAllActorsOfClass "/Game/TalesContent/Blueprints/Actors/BP_Dungeon_Entrance.BP_Dungeon_Entrance_C"))
  (for _array_element _outactors
    (Default|CreatePortal _array_element)))

(fn ConstructionScript)

(fn GetDungeonSpawn
  (bind _pcgactor (Variables|Default|GetPcgActor)
    (:then
      (return (Transformation|GetActorLocation _pcgactor) (Transformation|GetActorRotation _pcgactor)))
    (:else
      (return "0, 0, 0" "0, 0, 0"))))

(fn SendPlayertoDungeon
  (params (Target :type Actor%20Object%20Reference))
  (bind _pcgactor (Variables|Default|GetPcgActor)
    (:then
      (Utilities|IsValid Target
        (:Is%20Valid
          (Transformation|SetActorLocation Target (Transformation|GetActorLocation _pcgactor) false true)
          (Transformation|SetActorRotation Target (Transformation|GetActorRotation _pcgactor) true))
        (:Is%20Not%20Valid
          (Development|PrintString "Teleport Player Failed" true true "(R=1.000000,G=0.042541,B=0.000000,A=1.000000)" 5.0 :!label _label))))
    (:else
      (goto _label))))