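; BP_TalesHud is the player HUD that creates the casting, active effects and hotbar widgets.
; On BeginPlay or RestartHud it retries until it finds a PlayerCharacterBase, then builds the widgets.
; AbilityComponent cast-start and cancel events drive the casting widget, while the hotbar receives the character reference.
; Effects update logic is left unwired, and a restart removes only the casting widget before rebuilding all three.
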(event `InitializeTalesCharacter`
  (bind _returnvalue (`GameplayStatics.GetPlayerCharacter` 0))
  ;[0.04 0.04 0.04 0.6] Loops until the player character has been found
  ; Should be called anytime the player's pawn/character changes
  (`/Engine/EditorBlueprintResources/StandardMacros.IsValid` _returnvalue
    (:`Is Valid`
      (bind _asplayer_character_base (cast `PlayerCharacterBase` _returnvalue)
        (:`then`
          (set `self.CharacterReference` _asplayer_character_base)
          (`self.InitializeHudWdgets`))
        (:`CastFailed`
          (`KismetSystemLibrary.Delay` 0.2 :!label _label)
          (`self.InitializeTalesCharacter`))))
    (:`Is Not Valid`
      (goto _label))))

(event `RestartHud`
  (`self.InvalidateExistingHud`)
  (`self.InitializeTalesCharacter` :!label _label_2))

(event `SetupEventListenerForCasting`
  (bind _characterreference (`self.CharacterReference`)
    (:`then`
      (bind _abilitycomponent (`CharacterBase.AbilityComponent` _characterreference))
      (add `AbilityComponent.OnAbilityCanceled` _abilitycomponent (`|CreateDelegate` :!event `Callback_CancelCasting`))
      (add `AbilityComponent.OnAbilityCastStarted` _abilitycomponent (`|CreateDelegate` :!event `Callback_CastingTimer`)))
    (:`else`
      (`KismetSystemLibrary.Delay` 0.2)
      (`self.SetupEventListenerForCasting`))))

(event `self.ReceiveBeginPlay`
  (goto _label_2))

(event `InvalidateExistingHud`
  (bind _castingtimerwidget (`self.CastingTimerWidget`)
    (:`then`
      (`Widget.RemoveFromParent` _castingtimerwidget))
    (:`else`)))

(event `InitializeHudWdgets`
  (`|ExecutionSequence`
    (:`then_0`
      (bind _returnvalue (`|CreateWidget` "/Game/TalesContent/Widgets/HUD_Casting_Widget.HUD_Casting_Widget_C" (`GameplayStatics.GetPlayerController` 0)))
      (`UserWidget.AddToViewport` _returnvalue 0)
      (`UserWidget.SetAnchorsInViewport` _returnvalue (make `Anchors` (0.5 0.7) (0.5 0.7)))
      (`UserWidget.SetAlignmentInViewport` _returnvalue (0.5 0.5))
      (set `self.CastingTimerWidget` _returnvalue)
      (`self.SetupEventListenerForCasting`)
      (`self.SetupEventListenerForEffects`))
    (:`then_1`
      (bind _returnvalue_2 (`|CreateWidget` "/Game/TalesContent/Widgets/HUD_Effects_Widget.HUD_Effects_Widget_C" (`GameplayStatics.GetPlayerController` 0)))
      (`UserWidget.AddToViewport` _returnvalue_2 0)
      (`UserWidget.SetAnchorsInViewport` _returnvalue_2 (make `Anchors` (0.0 0.3) (0.0 0.3)))
      (`UserWidget.SetAlignmentInViewport` _returnvalue_2 (0.0 0.0))
      (set `self.ActiveEffectsWidget` _returnvalue_2))
    (:`then_2`
      (bind _returnvalue_3 (`|CreateWidget` "/Game/TalesContent/Widgets/HUD_Hotbar_Widget.HUD_Hotbar_Widget_C" (`GameplayStatics.GetPlayerController` 0) (`self.CharacterReference`)))
      (`UserWidget.AddToViewport` _returnvalue_3 0)
      (`UserWidget.SetAnchorsInViewport` _returnvalue_3 (make `Anchors` (0.5 0.95) (0.5 0.95)))
      (`UserWidget.SetAlignmentInViewport` _returnvalue_3 (0.5 1.0))
      (set `self.HotbarWidget` _returnvalue_3))))

(event `Callback_CancelCasting`
  (params (AbilityName :type Name) (FailureMessage :type String))
  (`/Game/TalesContent/Widgets/HUD_Casting_Widget.CancelCasting` (`self.CastingTimerWidget`)))

(event `Callback_CastingTimer`
  (params (AbilityName :type Name) (CastTime :type "Float (single-precision)"))
  (bind _castingtimerwidget (`self.CastingTimerWidget`)
    (:`then`
      (`/Game/TalesContent/Widgets/HUD_Casting_Widget.SetAbilityName` _castingtimerwidget AbilityName))
    (:`else`)))

(event `SetupEventListenerForEffects`)

(event `Callback_ActiveEffectsUpdated`)

(fn `UserConstructionScript`)