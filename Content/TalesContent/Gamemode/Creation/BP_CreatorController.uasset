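; BP_CreatorController is the player controller for the Creation game mode, handling the menu key.
; On press it backs out one layer at a time through the Tales HUD: it closes visible widgets first.
; Otherwise it clears the character's ability target, closing the target window, and only when nothing is targeted or no CharacterBase exists does it force open the main menu.
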(event `EnhancedInput|/Game/TalesContent/Inputs/Actions/IA_Menu_Key`
  (params (ActionValue :type Boolean) (ElapsedSeconds :type "Float (double-precision)") (TriggeredSeconds :type "Float (double-precision)") (InputAction :type "InputAction Object Reference" :default "/Game/TalesContent/Inputs/Actions/IA_Menu_Key.IA_Menu_Key"))
  (:`Started`
    (bind _asbp_tales_hud (cast `/Game/TalesContent/Gamemode/BP_TalesHud` (`self.GetHUD`)))
    (if (> (`KismetArrayLibrary.Array_Length` (`/Game/TalesContent/Gamemode/BP_TalesHud.GetAllVisibleWidgets` _asbp_tales_hud true)) 0)
      (`/Game/TalesContent/Gamemode/BP_TalesHud.CloseWidget` _asbp_tales_hud false)
      (else
        (bind _ascharacter_base (cast `CharacterBase` (`GameplayStatics.GetPlayerCharacter` 0))
          (:`then`
            (bind _abilitycomponent (`CharacterBase.AbilityComponent` _ascharacter_base))
            (`/Engine/EditorBlueprintResources/StandardMacros.IsValid` (`AbilityComponent.GetTargetedActor` _abilitycomponent)
              (:`Is Valid`
                (`AbilityComponent.SetTargetedActor` _abilitycomponent null) ; Set null target will close target window
              )
              (:`Is Not Valid`
                (`/Game/TalesContent/Gamemode/BP_TalesHud.ToggleMainMenu` _asbp_tales_hud true false :!label _label))))
          (:`CastFailed`
            (goto _label)))))))

(fn `UserConstructionScript`)