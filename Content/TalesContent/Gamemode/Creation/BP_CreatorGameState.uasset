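; Game state for the character creator, tracking the selected character and handling saved character data.
; BeginPlay sets the save meta name; selecting a character updates the creator-in-use flag (true for negative indices) and signals the change.
; Save and load calls delegate to SaveGameData, with SaveCharacterAsync left empty.
; CreateCharacter saves synchronously, then tells BP_CreatorHud to stop the creator or show an error.
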(event `self.ReceiveBeginPlay`
  (`self.SetSaveGameMetaName` "savedata"))

(fn `CreateCharacter`
  (params (CharacterName :type String))
  (bind _returnvalue (`PlayerController.GetHUD` (`GameplayStatics.GetPlayerController` 0)))
  (bind _returnvalue_2 (`self.SaveCurrentCharacterSync`))
  (if _returnvalue_2
    (bind _asbp_creator_hud (cast `/Game/TalesContent/Gamemode/Creation/BP_CreatorHud` _returnvalue))
    (`/Game/TalesContent/Gamemode/Creation/BP_CreatorHud.StopCharacterCreator` _asbp_creator_hud)
    (else
      (bind _asbp_creator_hud_2 (cast `/Game/TalesContent/Gamemode/Creation/BP_CreatorHud` _returnvalue))
      (`/Game/TalesContent/Gamemode/Creation/BP_CreatorHud.CharacterCreatorError` _asbp_creator_hud_2 "Error in BP_CreatorGameState"))))

(fn `GetAllSavedCharacters`
  (returns (ReturnValue :type "Array of String"))
  (return (`self.GetSavedCharacterNames`)))

(fn `GetSavedCharacterData`
  (params (SaveSlotName :type String))
  (returns (SaveData :type "SavedCharacter Object Reference"))
  (bind _savegamedata (`self.SaveGameData`)
    (:`then`
      (bind _returnvalue (`GlobalSaveData.GetSavedCharacterData` _savegamedata SaveSlotName))
      (return _returnvalue))
    (:`else`
      (return null))))

(fn `GetSelectedCharacterNumber`
  (returns (CharacterSelected :type Integer))
  (return (`self.CharacterSelected`)))

(fn `SaveCharacter`
  (params (SaveSlotName :type String))
  (bind _savegamedata (`self.SaveGameData`)
    (:`then`
      (bind _asplayer_character_base (cast `PlayerCharacterBase` (`GameplayStatics.GetPlayerCharacter` 0)))
      (`GlobalSaveData.SaveCharacter` _savegamedata _asplayer_character_base SaveSlotName))
    (:`else`)))

(fn `SaveCharacterAsync`)

(fn `SetSelectedCharacter`
  (params (CharacterSelected :type Integer))
  (bind _output_get (set `self.CharacterSelected` CharacterSelected))
  (set `self.bIsCreatorInUse` (< _output_get 0))
  (`self.OnCharacterSelected` _output_get))

(fn `UserConstructionScript`)